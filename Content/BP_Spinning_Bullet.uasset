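; BP_Spinning_Bullet is a short-lived projectile actor that flashes random colors and explodes on contact.
; On BeginPlay it sets its lifespan, plays a launch sound and creates a dynamic material instance for the bullet mesh.
; A looping timer calls SetMaterial to randomize that instance's Color parameter and reapply it.
; Any actor overlap destroys the bullet, plays an explosion sound and spawns HitParticle and Explosion actors at its transform.
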(event `self.ReceiveBeginPlay`
  (`self.SetLifeSpan` 5.0)
  (`GameplayStatics.PlaySound2D` "/Game/Assets/391660__jeckkech__projectile.391660__jeckkech__projectile" 1.0 1.0 0.0 null null)
  (bind _returnvalue (`PrimitiveComponent.CreateDynamicMaterialInstance` (`self.BulletMesh`) 0 "/Game/RandomColor.RandomColor" "None"))
  (set `self.DynamicMaterial` _returnvalue)
  (`KismetSystemLibrary.K2_SetTimerDelegate` (delegate `Color change`) 0.25 true)
  (`self.Set Material`))

(event `Color change`
  (`self.Set Material`))

(event `self.ReceiveActorBeginOverlap`
  (params (OtherActor :type "Actor Object Reference"))
  (bind _returnvalue (`self.GetTransform`))
  (`self.K2_DestroyActor`)
  (`GameplayStatics.PlaySound2D` "/Game/Assets/522209__kutejnikov__explosion.522209__kutejnikov__explosion" 1.0 1.0 0.0 null null)
  (`|SpawnActorFromClass` "/Game/HitParticle.HitParticle_C" _returnvalue "Undefined" "OverrideRootScale" null null)
  (`|SpawnActorFromClass` "/Game/Explosion.Explosion_C" _returnvalue "Undefined" "OverrideRootScale" null null))

(fn `Set Material`
  (bind _dynamicmaterial (`self.DynamicMaterial`))
  (`MaterialInstanceDynamic.SetVectorParameterValue` _dynamicmaterial "Color" (make `LinearColor` (`KismetMathLibrary.RandomFloatInRange` 0.0 1.0) (`KismetMathLibrary.RandomFloatInRange` 0.0 1.0) (`KismetMathLibrary.RandomFloatInRange` 0.0 1.0) 1.0))
  (`PrimitiveComponent.SetMaterial` (`self.BulletMesh`) 0 _dynamicmaterial))

(fn `UserConstructionScript`)